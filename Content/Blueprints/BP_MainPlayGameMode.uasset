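; BP_MainPlayGameMode is the main play game mode, providing random item drops and the credits sequence.
; SpawnItem makes one cumulative-probability roll over DT_Items drop rates, spawning at most one BP_Money or BP_Item with a random count at the given location.
; PlayCredit plays the credits level sequence, shows the credit widget, disables player input and turns off the HUD.
; BeginPlay and Tick are empty.
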(event EventBeginPlay)

(event EventTick
  (params (DeltaSeconds :type Float%20%28single-precision%29)))

(fn ConstructionScript)

(fn SpawnItem
  (params (Location :type Vector))
  (LocalVariables|SetRandom (Math|Random|RandomFloat))
  (LocalVariables|SetRandom%20Count 0.0)
  (bind _outrownames (DataTable|GetDataTableRowNames "/Game/Assets/Data/Item/DT_Items.DT_Items"))
  (bind _array_element (Utilities|Array|ForEachLoopwithBreak _outrownames)
    (:LoopBody
      (bind _returnvalue (Utilities|GetDataTableRow "/Game/Assets/Data/Item/DT_Items.DT_Items" _array_element)
        (:then
          (if (> (.droprate _returnvalue) 0.0)
            (bind _output_get (LocalVariables|SetRandom%20Count (+ (LocalVariables|GetRandom%20Count) (.droprate _returnvalue))))
            (if (>= _output_get (LocalVariables|GetRandom))
              (if (Utilities|Enum|Equal(Enum) (.itemcode _returnvalue) "Money")
                (bind _returnvalue_2 (Game|SpawnActorfromClass "/Game/Blueprints/Actor/Item/BP_Money.BP_Money_C" (Math|Transform|MakeTransform Location "0, 0, 0" "1.000000,1.000000,1.000000") "Undefined" "MultiplyWithRoot" 0 0))
                (Variables|/Script/BiohazardRe4.BItem|SetCount _returnvalue_2 (Math|Random|RandomIntegerinRange (.mindropcount _returnvalue) (.maxdropcount _returnvalue)))
                (Default|SetCount _returnvalue_2)
                (else
                  (bind _returnvalue_3 (Game|SpawnActorfromClass "/Game/Blueprints/Actor/Item/BP_Item.BP_Item_C" (Math|Transform|MakeTransform Location "0, 0, 0" "1.000000,1.000000,1.000000") "Undefined" "MultiplyWithRoot" 0 0))
                  (Default|ItemSetting _returnvalue_3 (.itemcode _returnvalue) (Math|Random|RandomIntegerinRange (.mindropcount _returnvalue) (.maxdropcount _returnvalue)))))
              (return))))))))

(fn PlayCredit
  (bind _returnvalue (Game|GetPlayerController 0))
  (bind _returnvalue_2 (Sequencer|Player|CreateLevelSequencePlayer "/Game/Blueprints/Event/Credits/LS_CreditsLevelSequence.LS_CreditsLevelSequence"))
  (Sequencer|Player|Play _returnvalue_2 :!class /Script/MovieScene.MovieSceneSequencePlayer)
  (bind _returnvalue_3 (UserInterface|CreateWidget "/Game/Blueprints/Event/Credits/WBP_CreditWidget.WBP_CreditWidget_C"))
  (UserInterface|Viewport|AddtoViewport _returnvalue_3 0)
  (Input|DisableInput (Game|GetPlayerCharacter 0) _returnvalue)
  (bind _asbp_player_hud (Utilities|Casting|CastToBP_PlayerHUD (HUD|GetHUD _returnvalue)))
  (Default|OffHUD _asbp_player_hud))