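; Inventory weapon Blueprint that displays its loaded ammo count on an attached WBP_ItemNum widget.
; BeginPlay casts and caches the widget component's user widget.
; SetItemNumText offsets the widget component in proportion to item size, writes the loaded ammo, and colors it green at or above max ammo, white otherwise.
; OffItemNumText turns the text off through the widget's OffText.
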(event EventBeginPlay
  (bind _aswbp_item_num (Utilities|Casting|CastToWBP_ItemNum (UserInterface|GetWidget (Variables|Default|GetWidget))))
  (Variables|Default|SetWBP%20Item%20Num _aswbp_item_num))

(event Collision|EventActorBeginOverlap
  (params (OtherActor :type Actor%20Object%20Reference)))

(event EventTick
  (params (DeltaSeconds :type Float%20%28single-precision%29)))

(event EventSetItemNumText
  (bind _returnvalue (Class|BInventoryItem|GetItemSize))
  (bind _returnvalue_2 (Class|BInventoryWeapon|GetLoadedAmmo))
  (Transformation|SetRelativeLocation (Variables|Default|GetWidget) (Math|Vector|MakeVector (* (Math|Conversions|ToFloat(Integer) (.x _returnvalue)) 5.0) (* (Math|Conversions|ToFloat(Integer) (.y _returnvalue)) 5.0) 0.0) false false)
  (Default|SetTextNum (Variables|Default|GetWBP%20Item%20Num) _returnvalue_2)
  (if (>= _returnvalue_2 (Class|BInventoryWeapon|GetMaxAmmo))
    (Default|SetTextColor (Variables|Default|GetWBP%20Item%20Num) "(R=0.000000,G=1.000000,B=0.000000,A=1.000000)")
    (else
      (Default|SetTextColor (Variables|Default|GetWBP%20Item%20Num) "(R=1.000000,G=1.000000,B=1.000000,A=1.000000)"))))

(event EventOffItemNumText
  (Default|OffText (Variables|Default|GetWBP%20Item%20Num)))

(fn ConstructionScript)