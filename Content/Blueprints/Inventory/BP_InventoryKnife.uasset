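; BP_InventoryKnife is the inventory item Blueprint for a knife, showing a durability indicator through a widget component.
; BeginPlay casts the component's widget to WBP_ItemDurability and caches it.
; SetItemNumText repositions the widget according to the item's grid size and passes it the current durability percent, in place of setting count text.
; OffItemNumText is implemented empty, so it leaves the indicator untouched.
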(event EventBeginPlay
  (bind _aswbp_item_durability (Utilities|Casting|CastToWBP_ItemDurability (UserInterface|GetWidget (Variables|Default|GetWidget))))
  (Variables|Default|SetWidget%20Durability _aswbp_item_durability))

(event Collision|EventActorBeginOverlap
  (params (OtherActor :type Actor%20Object%20Reference)))

(event EventTick
  (params (DeltaSeconds :type Float%20%28single-precision%29)))

(event EventSetItemNumText
  (bind _returnvalue (Class|BInventoryItem|GetItemSize))
  (Transformation|SetRelativeLocation (Variables|Default|GetWidget) (Math|Vector|MakeVector (* (Math|Conversions|ToFloat(Integer) (.x _returnvalue)) 5.0) (* (Math|Conversions|ToFloat(Integer) (.y _returnvalue)) 5.0) 0.0) false false)
  (Default|SetDurability (Variables|Default|GetWidget%20Durability) (Class|BInventoryWeapon|GetDurabilityPercent)))

(event EventOffItemNumText)

(fn ConstructionScript)