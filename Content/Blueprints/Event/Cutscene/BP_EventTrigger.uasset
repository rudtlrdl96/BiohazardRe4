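; One-shot box trigger that starts a level sequence cutscene with the player character, Leon.
; On any overlap it disables input and collision, empties the weapon, freezes movement in Flying mode and plays the sequence with Leon bound by tag.
; Meanwhile Tick quickly lerps Leon to the target transform.
; A fixed delay, independent of sequence completion, then moves Leon to a hard-coded transform and restores state, collision, walking and input.
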(event OnComponentBeginOverlap(Box)
  (params (OverlappedComponent :type Primitive%20Component%20Object%20Reference) (OtherActor :type Actor%20Object%20Reference) (OtherComp :type Primitive%20Component%20Object%20Reference) (OtherBodyIndex :type Integer) (bFromSweep :type Boolean) (SweepResult :type Hit%20Result%20Structure%20%28by%20ref%29))
  (bind _bp_player_leon (Variables|Default|GetBP%20Player%20Leon))
  (bind _bp_player_leon_2 (Variables|Default|GetBP%20Player%20Leon))
  (bind _bp_player_leon_3 (Variables|Default|GetBP%20Player%20Leon))
  (bind _charactermovement (Variables|/Script/Engine.Character|GetCharacterMovement _bp_player_leon_3))
  (Input|DisableInput (Game|GetPlayerCharacter 0) (Game|GetPlayerController 0))
  (Collision|SetCollisionEnabled (Variables|Default|GetBox) "NoCollision")
  (Class|BLeon|ChangeUseWeapon _bp_player_leon_3 "Empty")
  (Variables|/Script/Engine.MovementComponent|SetVelocity _charactermovement "0, 0, 0")
  (Pawn|Components|CharacterMovement|SetMovementMode _charactermovement "MOVE_Flying" 0)
  (Collision|SetCollisionEnabled (Variables|/Script/Engine.Character|GetCapsuleComponent _bp_player_leon_3) "NoCollision")
  (Class|BLeon|SetCurrentFSMState _bp_player_leon_3 "CutScene00")
  (Variables|Default|SetStart%20Position (Transformation|GetActorLocation _bp_player_leon_3))
  (Variables|Default|SetStart%20Rotation (Transformation|GetActorRotation _bp_player_leon_3))
  (Variables|Default|SetIsStart true)
  (Variables|Default|SetTimer 0.0)
  (Class|LevelSequenceActor|SetBindingbyTag (Variables|Default|GetLevelSequnce) "Leon" (Utilities|Array|MakeArray (Game|GetPlayerCharacter 0)) true)
  (Sequencer|Player|Play (Variables|/Script/LevelSequence.LevelSequenceActor|GetSequencePlayer (Variables|Default|GetLevelSequnce)) :!class /Script/MovieScene.MovieSceneSequencePlayer)
  (Utilities|FlowControl|Delay 1e+01)
  (Transformation|SetActorLocation _bp_player_leon "342.640000,-1148.120000,91.000000" false false)
  (Transformation|SetActorRotation _bp_player_leon "0.000000,-40.100000,0.000000")
  (Class|BLeon|SetCurrentFSMState _bp_player_leon "Idle")
  (Collision|SetCollisionEnabled (Variables|/Script/Engine.Character|GetCapsuleComponent _bp_player_leon_2) "QueryAndPhysics")
  (Pawn|Components|CharacterMovement|SetMovementMode (Variables|/Script/Engine.Character|GetCharacterMovement _bp_player_leon_2) "MOVE_Walking" 0)
  (Input|EnableInput (Game|GetPlayerCharacter 0) (Game|GetPlayerController 0)))

(event EventBeginPlay
  (bind _asbp_player_leon (Utilities|Casting|CastToBP_Player_Leon (Game|GetPlayerCharacter 0)))
  (Variables|Default|SetBP%20Player%20Leon _asbp_player_leon))

(event Collision|EventActorBeginOverlap
  (params (OtherActor :type Actor%20Object%20Reference)))

(event EventTick
  (params (DeltaSeconds :type Float%20%28single-precision%29))
  (bind _bp_player_leon (Variables|Default|GetBP%20Player%20Leon))
  (bind _bp_player_leon_2 (Variables|Default|GetBP%20Player%20Leon))
  (if (Variables|Default|GetIsStart)
    (bind _output_get (Variables|Default|SetTimer (+ (* DeltaSeconds 5.0) (Variables|Default|GetTimer))))
    (if (> _output_get 1.0)
      (Variables|Default|SetIsStart false)
      (Transformation|SetActorLocation _bp_player_leon_2 (Variables|Default|GetTarget%20Position) false true)
      (Transformation|SetActorRotation _bp_player_leon_2 (Variables|Default|GetTarget%20Rotation))
      (else
        (Transformation|SetActorLocation _bp_player_leon (Math|Vector|Lerp(Vector) (Variables|Default|GetStart%20Position) (Variables|Default|GetTarget%20Position) (Variables|Default|GetTimer)) false true)
        (Transformation|SetActorRotation _bp_player_leon (Math|Rotator|Lerp(Rotator) (Variables|Default|GetStart%20Rotation) (Variables|Default|GetTarget%20Rotation) (Variables|Default|GetTimer) true) true)))))

(fn ConstructionScript)