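; BP_Money is a money pickup actor that displays its amount through a WBP_MoneyInteraction widget component.
; BeginPlay caches that widget, passes it the Count and marks the item as pickable.
; EnableInteractionUI turns on the widget's interaction state, and Set Count pushes the current Count to it.
; PickUpEvent flags the item as picked up, waits briefly, then destroys the actor and plays a 2D UI sound.
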(event EventBeginPlay
  (bind _aswbp_money_interaction (Utilities|Casting|CastToWBP_MoneyInteraction (UserInterface|GetWidget (Variables|Default|GetWidget))))
  (bind _output_get (Variables|Default|SetInteraction%20Widget _aswbp_money_interaction))
  (Default|SetCount _output_get (Variables|Default|GetCount))
  (Variables|Default|SetbCanPickup true))

(event Collision|EventActorBeginOverlap
  (params (OtherActor :type Actor%20Object%20Reference)))

(event EventTick
  (params (DeltaSeconds :type Float%20%28single-precision%29)))

(event EventEnableInteractionUI
  (Default|EnableInteraction (Variables|Default|GetInteraction%20Widget)))

(event EventPickUpEvent
  (Variables|Default|SetbIsPickup true)
  (Utilities|FlowControl|Delay 0.3)
  (Actor|DestroyActor)
  (Audio|PlaySound2D "/Game/Assets/UI/Sound/Ingame/SW_UI_Ingame_116.SW_UI_Ingame_116" 1.0 1.0 0.0 0 0))

(fn ConstructionScript)

(fn SetCount
  (Default|SetCount (Variables|Default|GetInteraction%20Widget) (Variables|Default|GetCount)))