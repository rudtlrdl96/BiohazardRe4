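; World pickup item actor whose mesh, name and icon come from DT_Items, found by looping rows to match ItemCode.
; The construction script sets the mesh; BeginPlay and ItemSetting also fill its WBP_ItemInteraction widget, including count.
; CheckInventory asks BP_Player_Leon's inventory for room, setting CanPickup and the widget's full-inventory state.
; PickUpEvent flags pickup, destroys the actor after a short delay and plays a sound; ItemOn and ItemOff toggle collision.
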(event EventBeginPlay
  (bind _aswbp_item_interaction (Utilities|Casting|CastToWBP_ItemInteraction (UserInterface|GetWidget (Variables|Default|GetWidget))))
  (bind _output_get (Variables|Default|SetItem%20Interaction%20Widget _aswbp_item_interaction))
  (Variables|/Game/Blueprints/Actor/Item/WBP_ItemInteraction.WBP_ItemInteraction_C|SetItem%20Actor _output_get self)
  (CallFunction|WidgetSetting))

(event Collision|EventActorBeginOverlap
  (params (OtherActor :type Actor%20Object%20Reference)))

(event EventTick
  (params (DeltaSeconds :type Float%20%28single-precision%29)))

(event EventEnableInteractionUI
  (Default|EnableInteraction (Variables|Default|GetItem%20Interaction%20Widget)))

(event EventPickUpEvent
  (Variables|Default|SetbIsPickup true)
  (Utilities|FlowControl|Delay 0.3)
  (Actor|DestroyActor)
  (Audio|PlaySound2D "/Game/Assets/UI/Sound/Ingame/SW_UI_Ingame_141.SW_UI_Ingame_141" 1.0 1.0 0.0 0 0))

(fn ConstructionScript
  (CallFunction|MeshSetting))

(fn CheckInventory
  (bind _asbp_player_leon (Utilities|Casting|CastToBP_Player_Leon (Game|Player|GetPlayerPawn 0)))
  (bind _returnvalue (Class|BInventoryActor|IsEmptySlot (Class|BLeon|GetInventoryActor _asbp_player_leon) (Variables|Default|GetItemCode) (Variables|Default|GetCount)))
  (bind _output_get (Variables|Default|SetbCanPickup _returnvalue))
  (Default|SetIsInventoryFull (Variables|Default|GetItem%20Interaction%20Widget) (not _output_get)))

(fn ItemSetting
  (params (Item%20Code :type EItemCode%20Enum :default "Empty") (Count :type Integer))
  (Variables|Default|SetItemCode Item%20Code)
  (Variables|Default|SetCount Count)
  (CallFunction|MeshSetting)
  (CallFunction|WidgetSetting))

(fn Itemon
  (Collision|SetCollisionEnabled (Variables|Default|GetCollision) "QueryAndPhysics"))

(fn ItemOff
  (Collision|SetCollisionEnabled (Variables|Default|GetCollision) "NoCollision"))

(fn MeshSetting
  (bind _outrownames (DataTable|GetDataTableRowNames "/Game/Assets/Data/Item/DT_Items.DT_Items"))
  (bind _array_element (Utilities|Array|ForEachLoopwithBreak _outrownames :!label _label)
    (:LoopBody
      (bind _returnvalue (Utilities|GetDataTableRow "/Game/Assets/Data/Item/DT_Items.DT_Items" _array_element)
        (:then
          (if (Utilities|Enum|Equal(Enum) (.itemcode _returnvalue) (Variables|Default|GetItemCode))
            (Components|StaticMesh|SetStaticMesh (Variables|Character|GetMesh) (.mesh _returnvalue))
            (goto _label Break)))))))

(fn WidgetSetting
  (bind _item_interaction_widget (Variables|Default|GetItem%20Interaction%20Widget))
  (Default|SetCount (Variables|Default|GetItem%20Interaction%20Widget) (Variables|Default|GetCount))
  (bind _outrownames (DataTable|GetDataTableRowNames "/Game/Assets/Data/Item/DT_Items.DT_Items"))
  (for _array_element _outrownames
    (bind _returnvalue (Utilities|GetDataTableRow "/Game/Assets/Data/Item/DT_Items.DT_Items" _array_element)
      (:then
        (if (Utilities|Enum|Equal(Enum) (.itemcode _returnvalue) (Variables|Default|GetItemCode))
          (Default|SetItemName _item_interaction_widget (.itemname _returnvalue))
          (Default|SetItemIcon _item_interaction_widget (.icon _returnvalue)))))))