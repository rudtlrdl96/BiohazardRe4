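; BP_MonsterFemale is a female monster actor assembled from modular skeletal mesh parts, with an interaction widget.
; The construction script sets the main mesh as leader pose for the hat, head, pants and jacket so they animate together.
; On BeginPlay it caches its widget component's WBP_Interaction, which the EnableInteractionUI event uses to enable the interaction prompt.
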(event EventBeginPlay
  (bind _aswbp_interaction (Utilities|Casting|CastToWBP_Interaction (UserInterface|GetWidget (Variables|Default|GetWidget))))
  (Variables|Default|SetInteraction _aswbp_interaction))

(event Collision|EventActorBeginOverlap
  (params (OtherActor :type Actor%20Object%20Reference)))

(event EventTick
  (params (DeltaSeconds :type Float%20%28single-precision%29)))

(event EventEnableInteractionUI
  (Default|EnableInteraction (Variables|Default|GetInteraction)))

(fn ConstructionScript
  (Components|SkinnedMesh|SetLeaderPoseComponent (Variables|Default|GetHat) (Variables|Character|GetMesh) true true))