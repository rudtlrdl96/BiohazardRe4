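; Male patrol monster actor that shows player interaction prompts and drops an item on death.
; BeginPlay caches the enemy interaction widget and applies a shared Animation Blueprint class to the modular head, clothing and weapon meshes.
; Tick polls Stat for death, then disables itself and, after a delay, has the main game mode spawn an item below the actor.
; Events forward interaction and parry states to the widget, delaying parry-off briefly.
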(event EventBeginPlay
  (bind _aswbp_enemy_interaction (Utilities|Casting|CastToWBP_EnemyInteraction (UserInterface|GetWidget (Variables|Default|GetWidget))))
  (Variables|Default|SetInteraction _aswbp_enemy_interaction)
  (Class|SkeletalMeshComponent|SetAnimClass (Variables|Default|GetHead) "/Game/Blueprints/Actor/Monster/ABP_BasicMonsterMaleCopy.ABP_BasicMonsterMaleCopy_C")
  (Class|SkeletalMeshComponent|SetAnimClass (Variables|Default|GetJacket) "/Game/Blueprints/Actor/Monster/ABP_BasicMonsterMaleCopy.ABP_BasicMonsterMaleCopy_C")
  (Class|SkeletalMeshComponent|SetAnimClass (Variables|Default|GetPants) "/Game/Blueprints/Actor/Monster/ABP_BasicMonsterMaleCopy.ABP_BasicMonsterMaleCopy_C")
  (Class|SkeletalMeshComponent|SetAnimClass (Variables|Default|GetHat) "/Game/Blueprints/Actor/Monster/ABP_BasicMonsterMaleCopy.ABP_BasicMonsterMaleCopy_C")
  (Class|SkeletalMeshComponent|SetAnimClass (Variables|Default|GetWeapon) "/Game/Blueprints/Actor/Monster/ABP_BasicMonsterMaleCopy.ABP_BasicMonsterMaleCopy_C"))

(event Collision|EventActorBeginOverlap
  (params (OtherActor :type Actor%20Object%20Reference)))

(event EventTick
  (params (DeltaSeconds :type Float%20%28single-precision%29))
  (if (Class|BMonsterStatComponent|IsDeath (Variables|Default|GetStat))
    (Actor|Tick|SetActorTickEnabled false)
    (Utilities|FlowControl|Delay 2.0)
    (Development|PrintString "아이템 스폰")
    (bind _asbp_main_play_game_mode (Utilities|Casting|CastToBP_MainPlayGameMode (Game|GetGameMode)))
    (Default|SpawnItem _asbp_main_play_game_mode (+ (Transformation|GetActorLocation) "0.000000,0.000000,-88.000000"))))

(event EventEnableInteractionUI
  (Default|EnableInteraction (Variables|Default|GetInteraction)))

(event EventOnParryInteraction
  (Default|OnParryInteraction (Variables|Default|GetInteraction))
  (Development|PrintString "Hello"))

(event EventOffParryInteraction
  (Utilities|FlowControl|Delay 0.2)
  (Default|OffParryInteraction (Variables|Default|GetInteraction)))

(fn ConstructionScript)