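; BP_BMapDrawerInteraction is an interactable map drawer that holds a hidden item.
; On BeginPlay it caches its interaction widget, then spawns a BP_Item with a configured code and count, switched off and attached to the drawer's collision component.
; A trigger overlap toggles the interactable flag, and an event enables the interaction UI.
; Tick polls the Open flag, then turns the item on and clears the flag.
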(event OnComponentBeginOverlap(ATrigger)
  (params (OverlappedComponent :type Primitive%20Component%20Object%20Reference) (OtherActor :type Actor%20Object%20Reference) (OtherComp :type Primitive%20Component%20Object%20Reference) (OtherBodyIndex :type Integer) (bFromSweep :type Boolean) (SweepResult :type Hit%20Result%20Structure%20%28by%20ref%29))
  ;[1 1 1] 상호작용 가능 불가능
  (Variables|Default|SetbInter true))

(event OnComponentEndOverlap(ATrigger)
  (params (OverlappedComponent :type Primitive%20Component%20Object%20Reference) (OtherActor :type Actor%20Object%20Reference) (OtherComp :type Primitive%20Component%20Object%20Reference) (OtherBodyIndex :type Integer))
  ;[1 1 1] 상호작용 가능 불가능
  (Variables|Default|SetbInter false))

(event EventBeginPlay
  (bind _aswbp_interaction (Utilities|Casting|CastToWBP_Interaction (UserInterface|GetWidget (Variables|Default|GetWidget))))
  (Variables|Default|SetInteraction _aswbp_interaction)
  (bind _returnvalue (Game|SpawnActorfromClass "/Game/Blueprints/Actor/Item/BP_Item.BP_Item_C" (Math|Conversions|ToTransform(Vector) (Transformation|GetWorldLocation (Variables|Default|GetDrawerCol))) "Undefined" "MultiplyWithRoot" 0 0))
  (bind _output_get (Variables|Default|Setitem _returnvalue))
  (Default|ItemSetting _output_get (Variables|Item|GetItem%20Code) (Variables|Item|GetCount))
  (Default|ItemOff _output_get)
  (Transformation|AttachComponentToComponent (Variables|/Script/Engine.Actor|GetRootComponent (Variables|Default|Getitem)) (Variables|Default|GetDrawerCol) "None" "KeepWorld" "KeepWorld" "KeepWorld" true))

(event Collision|EventActorBeginOverlap
  (params (OtherActor :type Actor%20Object%20Reference)))

(event EventEnableInteractionUI
  (Default|EnableInteraction (Variables|Default|GetInteraction)))

(event EventTick
  (params (DeltaSeconds :type Float%20%28single-precision%29))
  (if (Variables|Default|GetbOpen)
    (Default|Itemon (Variables|Default|Getitem))
    (Variables|Default|SetbOpen false)))

(fn ConstructionScript)