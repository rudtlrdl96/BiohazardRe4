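; BP_Location01MonsterSpawn is a map trigger actor that spawns idle male monsters for Location 01 when its SpawnTrigger component is overlapped.
; If IsSpawn is true, a chain of one-second Delays staggers four BP_MonsterMale_Idle spawns at hard-coded positions.
; The overlap does not filter the entering actor.
; IsSpawn clears only after the final spawn, so overlaps during the sequence still pass the check.
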(event OnComponentBeginOverlap(SpawnTrigger)
  (params (OverlappedComponent :type Primitive%20Component%20Object%20Reference) (OtherActor :type Actor%20Object%20Reference) (OtherComp :type Primitive%20Component%20Object%20Reference) (OtherBodyIndex :type Integer) (bFromSweep :type Boolean) (SweepResult :type Hit%20Result%20Structure%20%28by%20ref%29))
  (if (Variables|Default|GetIsSpawn)
    (Utilities|FlowControl|Delay 1.0)
    (Game|SpawnActorfromClass "/Game/Blueprints/Actor/Monster/BP_MonsterMale_Idle.BP_MonsterMale_Idle_C" (Math|Conversions|ToTransform(Vector) "-9574.754009,3219.062784,462.487364") "Undefined" "MultiplyWithRoot" 0 0)
    (Utilities|FlowControl|Delay 1.0)
    (Game|SpawnActorfromClass "/Game/Blueprints/Actor/Monster/BP_MonsterMale_Idle.BP_MonsterMale_Idle_C" (Math|Conversions|ToTransform(Vector) "-9367.822652,3502.406633,562.141267") "Undefined" "MultiplyWithRoot" 0 0)
    (Utilities|FlowControl|Delay 1.0)
    (Game|SpawnActorfromClass "/Game/Blueprints/Actor/Monster/BP_MonsterMale_Idle.BP_MonsterMale_Idle_C" (Math|Conversions|ToTransform(Vector) "-8074.015443,3628.824005,706.479246") "Undefined" "MultiplyWithRoot" 0 0)
    (Utilities|FlowControl|Delay 1.0)
    (Game|SpawnActorfromClass "/Game/Blueprints/Actor/Monster/BP_MonsterMale_Idle.BP_MonsterMale_Idle_C" (Math|Conversions|ToTransform(Vector) "-7508.917559,2612.924808,445.845364") "Undefined" "MultiplyWithRoot" 0 0)
    (Variables|Default|SetIsSpawn false)))

(event Collision|EventActorBeginOverlap
  (params (OtherActor :type Actor%20Object%20Reference)))

(fn ConstructionScript)