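; BP_CullingCollision01 is an overlap volume actor that manually culls a map mesh based on the player's presence.
; Begin overlap with BP_Player_Leon shows the mesh's StaticMeshComponent, and end overlap hides it, without propagating to children.
; The target mesh is held in the MapMesh variable, assignable through the SetMapMesh function.
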(event Collision|EventActorEndOverlap
  (params (OtherActor :type Actor%20Object%20Reference))
  (Utilities|Casting|CastToBP_Player_Leon OtherActor)
  (Rendering|SetVisibility (Variables|/Script/Engine.StaticMeshActor|GetStaticMeshComponent (Variables|Default|GetMapMesh)) false false))

(event Collision|EventActorBeginOverlap
  (params (OtherActor :type Actor%20Object%20Reference))
  (Utilities|Casting|CastToBP_Player_Leon OtherActor)
  (Rendering|SetVisibility (Variables|/Script/Engine.StaticMeshActor|GetStaticMeshComponent (Variables|Default|GetMapMesh)) true false))

(fn ConstructionScript)

(fn SetMapMesh
  (params (MapMesh :type Static%20Mesh%20Actor%20Object%20Reference))
  (Variables|Default|SetMapMesh MapMesh))