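; Map actor for Location00 that stages two idle male monsters and reveals them when its trigger volume is entered.
; On BeginPlay it spawns both monsters at hard-coded world transforms and keeps references to them.
; An overlap on SpawnTrigger calls each monster's OnVisibilty, with no check on the overlapping actor, then clears IsSpawn so the reveal does not repeat.
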(event OnComponentBeginOverlap(SpawnTrigger)
  (params (OverlappedComponent :type Primitive%20Component%20Object%20Reference) (OtherActor :type Actor%20Object%20Reference) (OtherComp :type Primitive%20Component%20Object%20Reference) (OtherBodyIndex :type Integer) (bFromSweep :type Boolean) (SweepResult :type Hit%20Result%20Structure%20%28by%20ref%29))
  (if (Variables|Default|GetIsSpawn)
    (Default|OnVisibilty (Variables|Default|GetMonster00))
    (Default|OnVisibilty (Variables|Default|GetMonster01))
    (Variables|Default|SetIsSpawn false)))

(event EventBeginPlay
  (bind _returnvalue (Game|SpawnActorfromClass "/Game/Blueprints/Actor/Monster/BP_MonsterMale_Idle.BP_MonsterMale_Idle_C" (Math|Transform|MakeTransform "-12186.221709,5120.433575,811.800896" "0.000000,-112.983150,0.000000") "Undefined" "MultiplyWithRoot" 0 0))
  (Variables|Default|SetMonster00 _returnvalue)
  (bind _returnvalue_2 (Game|SpawnActorfromClass "/Game/Blueprints/Actor/Monster/BP_MonsterMale_Idle.BP_MonsterMale_Idle_C" (Math|Transform|MakeTransform "-10648.607475,5212.346104,820.747338" "0.000000,86.000000,0.000000") "Undefined" "MultiplyWithRoot" 0 0))
  (Variables|Default|SetMonster01 _returnvalue_2))

(fn ConstructionScript)