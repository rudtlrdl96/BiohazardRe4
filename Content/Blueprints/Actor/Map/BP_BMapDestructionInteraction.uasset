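; Breakable box map actor that holds a hidden item and reveals it when the box is damaged.
; BeginPlay spawns a BP_Item configured by item code and count, switches it off, and caches the interaction widget for EnableInteractionUI.
; The first damage swaps the Ork component for a runtime-added Geometry Collection pushed by radial impulses, plays a break sound, disables trigger collision and turns the item on.
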(event EventBeginPlay
  (bind _returnvalue (Game|SpawnActorfromClass "/Game/Blueprints/Actor/Item/BP_Item.BP_Item_C" (Transformation|GetActorTransform) "Undefined" "MultiplyWithRoot" 0 0))
  (bind _output_get (Variables|Default|SetItem _returnvalue))
  (Default|ItemSetting _output_get (Variables|Item|GetItem%20Code) (Variables|Item|GetCount))
  (Default|ItemOff _output_get)
  (bind _aswbp_interaction (Utilities|Casting|CastToWBP_Interaction (UserInterface|GetWidget (Variables|Default|GetWidget))))
  (Variables|Default|SetInteraction _aswbp_interaction))

(event EventEnableInteractionUI
  (Default|EnableInteraction (Variables|Default|GetInteraction)))

(event EventTick
  (params (DeltaSeconds :type Float%20%28single-precision%29)))

(event Game|Damage|EventAnyDamage
  (params (Damage :type Float%20%28single-precision%29) (DamageType :type Damage%20Type%20Object%20Reference) (InstigatedBy :type Controller%20Object%20Reference) (DamageCauser :type Actor%20Object%20Reference))
  (bind _returnvalue (Transformation|GetActorLocation))
  (if (not (Variables|Default|GetIsBroken))
    (Components|DestroyComponent (Variables|Default|GetOrk))
    (bind _returnvalue_2 (AddComponent|AddGeometryCollectionComponent false))
    (Physics|AddRadialImpulse _returnvalue_2 _returnvalue 1e+01 1e+01 "RIF_Linear" false)
    (Physics|AddRadialImpulse _returnvalue_2 _returnvalue 1e+01 1e+01 "RIF_Linear" false)
    (Audio|PlaySound2D "/Game/Assets/Map/Location01/Sound/SC_RandomBreakBox.SC_RandomBreakBox" 1.0 1.0 0.0 0 0)
    (Collision|SetCollisionEnabled (Variables|Default|GetATrigger) "NoCollision")
    (Variables|Default|SetIsBroken true)
    (Default|Itemon (Variables|Default|GetItem))))

(fn ConstructionScript)