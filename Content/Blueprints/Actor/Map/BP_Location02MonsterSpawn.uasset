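; Spawner actor for Location 02 that populates the map with male monsters and activates them when its trigger is overlapped.
; BeginPlay spawns seven patrol and three idle monsters at hardcoded transforms and stores each in its own variable.
; The first SpawnTrigger overlap while Isspawn is set calls each monster's visibility function, then clears the flag so it fires only once.
; The overlapping actor is not filtered.
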(event OnComponentBeginOverlap(SpawnTrigger)
  (params (OverlappedComponent :type Primitive%20Component%20Object%20Reference) (OtherActor :type Actor%20Object%20Reference) (OtherComp :type Primitive%20Component%20Object%20Reference) (OtherBodyIndex :type Integer) (bFromSweep :type Boolean) (SweepResult :type Hit%20Result%20Structure%20%28by%20ref%29))
  (if (Variables|Default|GetIsspawn)
    (Default|OnVisibity (Variables|Default|GetMonster00))
    (Default|OnVisibity (Variables|Default|GetMonster01))
    (Default|OnVisibity (Variables|Default|GetMonster02))
    (Default|OnVisibity (Variables|Default|GetMonster03))
    (Default|OnVisibity (Variables|Default|GetMonster04))
    (Default|OnVisibity (Variables|Default|GetMonster05))
    (Default|OnVisibity (Variables|Default|GetMonster06))
    (Default|OnVisibilty (Variables|Default|GetMonster07))
    (Default|OnVisibilty (Variables|Default|GetMonster08))
    (Default|OnVisibilty (Variables|Default|GetMonster09))
    (Variables|Default|SetIsspawn false)))

(event EventBeginPlay
  (bind _returnvalue (Game|SpawnActorfromClass "/Game/Blueprints/Actor/Monster/BP_MonsterMale_Patrol.BP_MonsterMale_Patrol_C" (Math|Transform|MakeTransform "-1015.784118,-83.971306,87.950995" "0.000000,180.000000,0.000000") "Undefined" "MultiplyWithRoot" 0 0))
  (Variables|Default|SetMonster00 _returnvalue)
  (bind _returnvalue_2 (Game|SpawnActorfromClass "/Game/Blueprints/Actor/Monster/BP_MonsterMale_Patrol.BP_MonsterMale_Patrol_C" (Math|Transform|MakeTransform "-663.111213,6.279436,83.729195" "0.000000,180.000000,0.000000") "Undefined" "MultiplyWithRoot" 0 0))
  (Variables|Default|SetMonster01 _returnvalue_2)
  (bind _returnvalue_3 (Game|SpawnActorfromClass "/Game/Blueprints/Actor/Monster/BP_MonsterMale_Patrol.BP_MonsterMale_Patrol_C" (Math|Conversions|ToTransform(Vector) "-336.021329,40.411965,75.237715") "Undefined" "MultiplyWithRoot" 0 0))
  (Variables|Default|SetMonster02 _returnvalue_3)
  (bind _returnvalue_4 (Game|SpawnActorfromClass "/Game/Blueprints/Actor/Monster/BP_MonsterMale_Patrol.BP_MonsterMale_Patrol_C" (Math|Conversions|ToTransform(Vector) "1310.854275,-150.749366,87.407332") "Undefined" "MultiplyWithRoot" 0 0))
  (Variables|Default|SetMonster03 _returnvalue_4)
  (bind _returnvalue_5 (Game|SpawnActorfromClass "/Game/Blueprints/Actor/Monster/BP_MonsterMale_Patrol.BP_MonsterMale_Patrol_C" (Math|Transform|MakeTransform "-349.549629,364.839278,84.082769" "0.000000,180.000000,0.000000") "Undefined" "MultiplyWithRoot" 0 0))
  (Variables|Default|SetMonster04 _returnvalue_5)
  (bind _returnvalue_6 (Game|SpawnActorfromClass "/Game/Blueprints/Actor/Monster/BP_MonsterMale_Patrol.BP_MonsterMale_Patrol_C" (Math|Conversions|ToTransform(Vector) "259.081920,-298.813383,80.746617") "Undefined" "MultiplyWithRoot" 0 0))
  (Variables|Default|SetMonster05 _returnvalue_6)
  (bind _returnvalue_7 (Game|SpawnActorfromClass "/Game/Blueprints/Actor/Monster/BP_MonsterMale_Patrol.BP_MonsterMale_Patrol_C" (Math|Conversions|ToTransform(Vector) "438.988021,114.700152,92.837982") "Undefined" "MultiplyWithRoot" 0 0))
  (Variables|Default|SetMonster06 _returnvalue_7)
  (bind _returnvalue_8 (Game|SpawnActorfromClass "/Game/Blueprints/Actor/Monster/BP_MonsterMale_Idle.BP_MonsterMale_Idle_C" (Math|Conversions|ToTransform(Vector) "-2304.246498,-752.023101,98.891219") "Undefined" "MultiplyWithRoot" 0 0))
  (Variables|Default|SetMonster07 _returnvalue_8)
  (bind _returnvalue_9 (Game|SpawnActorfromClass "/Game/Blueprints/Actor/Monster/BP_MonsterMale_Idle.BP_MonsterMale_Idle_C" (Math|Conversions|ToTransform(Vector) "-1694.024531,-961.600035,110.913607") "Undefined" "MultiplyWithRoot" 0 0))
  (Variables|Default|SetMonster08 _returnvalue_9)
  (bind _returnvalue_10 (Game|SpawnActorfromClass "/Game/Blueprints/Actor/Monster/BP_MonsterMale_Idle.BP_MonsterMale_Idle_C" (Math|Conversions|ToTransform(Vector) "-118.823275,-2291.374244,95.538871") "Undefined" "MultiplyWithRoot" 0 0))
  (Variables|Default|SetMonster09 _returnvalue_10))

(fn ConstructionScript)