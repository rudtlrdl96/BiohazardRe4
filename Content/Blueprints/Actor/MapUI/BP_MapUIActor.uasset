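; BP_MapUIActor is a map UI actor that paints fog of war around the player's marker.
; On BeginPlay it creates dynamic cover and reveal materials and clears both render targets to black.
; Each tick, a short downward trace at PlayerWidget finds the hit UV, which sets the cover material's Location before it is drawn into RT_FOWReveal.
; The reveal material instance is stored but unused in these graphs.
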(event EventBeginPlay
  (bind _returnvalue (Rendering|Material|CreateDynamicMaterialInstance "/Game/Assets/UI/MapUI/FogOfWar/M_FOWCover.M_FOWCover" "None" "None" :!class /Script/Engine.KismetMaterialLibrary))
  (Variables|Default|SetFOWCoverMat _returnvalue)
  (bind _returnvalue_2 (Rendering|Material|CreateDynamicMaterialInstance "/Game/Assets/UI/MapUI/FogOfWar/M_FOWReveal.M_FOWReveal" "None" "None" :!class /Script/Engine.KismetMaterialLibrary))
  (Variables|Default|SetFOWRevealMat _returnvalue_2)
  (Rendering|ClearRenderTarget2D "/Game/Assets/UI/MapUI/FogOfWar/RT_FOWCover.RT_FOWCover")
  (Rendering|ClearRenderTarget2D "/Game/Assets/UI/MapUI/FogOfWar/RT_FOWReveal.RT_FOWReveal"))

(event EventTick
  (params (DeltaSeconds :type Float%20%28single-precision%29))
  (bind _playerwidget (Variables|Default|GetPlayerWidget))
  (bind _returnvalue (Transformation|GetWorldLocation _playerwidget))
  (bind _outhit (Collision|LineTraceByChannel (+ _returnvalue "0.000000,0.000000,5.000000") (+ _returnvalue "") "TraceTypeQuery4" true 0 "None" false))
  (Rendering|Material|SetVectorParameterValue (Variables|Default|GetFOWCoverMat) "Location" (Utilities|Struct|MakeLinearColor (.x (.UV (Class|GameplayStatics|FindCollisionUV _outhit))) (.y (.UV (Class|GameplayStatics|FindCollisionUV _outhit))) 0.0 1.0) :!class /Script/Engine.MaterialInstanceDynamic)
  (Rendering|DrawMaterialtoRenderTarget "/Game/Assets/UI/MapUI/FogOfWar/RT_FOWReveal.RT_FOWReveal" (Variables|Default|GetFOWCoverMat)))

(fn ConstructionScript)