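; BP_PlayerHUD creates the player's HUD widget and relays health, heal preview, weapon, ammo and knife updates to it.
; On BeginPlay it adds WBP_PlayerHUD to the viewport and caches its quick-slot panel, though QuickSlotUpdate is still empty.
; When the widget's HP or knife durability setters return true, Timelines here drive its damage animations through per-update and end callbacks.
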(event EventBeginPlay
  (bind _returnvalue (UserInterface|CreateWidget "/Game/Blueprints/Actor/PlayerUI/WBP_PlayerHUD.WBP_PlayerHUD_C"))
  (bind _output_get (Variables|Default|SetWidget%20Ref _returnvalue))
  (UserInterface|Viewport|AddtoViewport _output_get 0)
  (bind _quick_slot (Default|GetQuickSlotPanel _output_get))
  (Variables|Default|SetQuickSlot%20Widget _quick_slot))

(event Collision|EventActorBeginOverlap
  (params (OtherActor :type Actor%20Object%20Reference)))

(event EventQuickSlotUpdate)

(event EventSetHealPreview
  (params (Percent :type Float%20%28single-precision%29))
  (Default|SetHealPreview (Variables|Default|GetWidget%20Ref) Percent))

(event EventOffHealPreview
  (Default|OffHealPreview (Variables|Default|GetWidget%20Ref)))

(event EventTick
  (params (DeltaSeconds :type Float%20%28single-precision%29)))

(event EventSetMaxHP
  (params (Percent :type Float%20%28single-precision%29))
  (Default|SetMaxHP (Variables|Default|GetWidget%20Ref) Percent))

(event EventSetKnife
  (params (IsVisible :type Boolean))
  (Default|SetKnife (Variables|Default|GetWidget%20Ref) IsVisible))

(event EventSetKnifeDurability
  (params (Durability :type Float%20%28single-precision%29))
  (bind _widget_ref (Variables|Default|GetWidget%20Ref))
  (bind _isdamage (Default|SetKnifeDurability (Variables|Default|GetWidget%20Ref) Durability))
  (if _isdamage
    (bind _curve (Timeline|타임라인 PlayFromStart)
      (:Update
        (Default|SetKnifeDamageUpdate _widget_ref _curve))
      (:Finished
        (Default|SetKnifeDamageEnd _widget_ref)))))

(event EventSetLoadAmmo
  (params (Ammo :type Integer))
  (Default|SetLoadedAmmo (Variables|Default|GetWidget%20Ref) Ammo))

(event EventSetHP
  (params (Percent :type Float%20%28single-precision%29))
  (bind _widget_ref (Variables|Default|GetWidget%20Ref))
  (bind _isdamage (Default|SetHP (Variables|Default|GetWidget%20Ref) Percent))
  (if _isdamage
    ;[1 1 1] Damage
    (bind _curve (Timeline|타임라인_0 PlayFromStart)
      (:Update
        (Default|SetHPDamageUpdate _widget_ref _curve))
      (:Finished
        (Default|SetHPDamageEnd _widget_ref)))))

(event EventSetWeapon
  (params (Weapon :type B%20Inventory%20Weapon%20Object%20Reference))
  (Default|SetWeapon (Variables|Default|GetWidget%20Ref) Weapon))

(event EventSetStoredAmmo
  (params (Ammo :type Integer))
  (Default|SetStoredAmmo (Variables|Default|GetWidget%20Ref) Ammo))

(fn ConstructionScript)