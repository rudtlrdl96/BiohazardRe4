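; Merchant NPC actor that shows a prompt when BP_Player_Leon enters its sphere and opens a store on F.
; Opening creates WBP_Store, switches to UI input and the merchant's camera, and sets an animation state; closing reverses this.
; Exposed functions toggle two cameras and preview items using mesh and transform from DT_Items.
; The construction script makes mask and face follow the body's pose.
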(event OnComponentBeginOverlap(Sphere)
  (params (OverlappedComponent :type Primitive%20Component%20Object%20Reference) (OtherActor :type Actor%20Object%20Reference) (OtherComp :type Primitive%20Component%20Object%20Reference) (OtherBodyIndex :type Integer) (bFromSweep :type Boolean) (SweepResult :type Hit%20Result%20Structure%20%28by%20ref%29))
  (if (== (Utilities|GetClass OtherActor) "/Game/Blueprints/Actor/Player/BP_Player_Leon.BP_Player_Leon_C")
    (Rendering|SetVisibility (Variables|Default|GetWidget) true false)
    (Variables|Default|SetIs%20Overlap true)))

(event OnComponentEndOverlap(Sphere)
  (params (OverlappedComponent :type Primitive%20Component%20Object%20Reference) (OtherActor :type Actor%20Object%20Reference) (OtherComp :type Primitive%20Component%20Object%20Reference) (OtherBodyIndex :type Integer))
  (if (== (Utilities|GetClass OtherActor) "/Game/Blueprints/Actor/Player/BP_Player_Leon.BP_Player_Leon_C")
    (Rendering|SetVisibility (Variables|Default|GetWidget) false false)
    (Variables|Default|SetIs%20Overlap false)))

(event Custom|Preview%20Item
  (params (ItemRowName :type Name))
  (bind _itemmesh (Variables|Default|GetItemMesh))
  (bind _returnvalue (Utilities|GetDataTableRow "/Game/Assets/Data/Item/DT_Items.DT_Items" ItemRowName)
    (:then
      (Components|StaticMesh|SetStaticMesh _itemmesh (.mesh _returnvalue))
      (Transformation|SetRelativeLocation _itemmesh (.storelocation _returnvalue) false false)
      (Transformation|SetRelativeRotation _itemmesh (.storerotation _returnvalue) false false)
      (Transformation|SetRelativeScale3D _itemmesh (.storescale _returnvalue))
      (Rendering|SetVisibility _itemmesh true false))))

(event EventBeginPlay)

(event Collision|EventActorBeginOverlap
  (params (OtherActor :type Actor%20Object%20Reference)))

(event EventTick
  (params (DeltaSeconds :type Float%20%28single-precision%29)))

(event Input|KeyboardEvents|F
  (params (Key :type Key%20Structure))
  (:Pressed
    (if (Variables|Default|GetIs%20Overlap)
      (CallFunction|OpenStore))))

(fn ConstructionScript
  (Components|SkinnedMesh|SetLeaderPoseComponent (Variables|Default|GetMask) (Variables|Default|GetBody) false false))

(fn SetCameraDefault
  (Components|Activation|SetActive (Variables|Default|GetCamera) true false)
  (Components|Activation|SetActive (Variables|Default|GetCamera1) false false))

(fn SetCameraSecond
  (Components|Activation|SetActive (Variables|Default|GetCamera) false false)
  (Components|Activation|SetActive (Variables|Default|GetCamera1) true false))

(fn CloseStore
  (bind _returnvalue (Game|GetPlayerController 0))
  (Widget|SetVisibility (UserInterface|GetWidget (Variables|Default|GetWidget)) "Visible")
  (Widget|RemovefromParent (Variables|Default|GetStore%20Widget))
  (Input|SetInputModeGameOnly _returnvalue false)
  (Variables|/Script/Engine.PlayerController|SetbShowMouseCursor _returnvalue false)
  (Game|Player|SetViewTargetwithBlend _returnvalue (Game|GetPlayerCharacter 0) 0.0 "VTBlend_Linear" 0.0 false)
  (Variables|Default|SetState "Idle"))

(fn OpenStore
  (bind _returnvalue (Game|GetPlayerController 0))
  (Widget|SetVisibility (UserInterface|GetWidget (Variables|Default|GetWidget)) "Hidden") ; F 키 입력 UI를 끔
  (bind _returnvalue_2 (UserInterface|CreateWidget "/Game/Blueprints/Actor/Merchant/WBP_Store.WBP_Store_C"))
  (bind _output_get (Variables|Default|SetStore%20Widget _returnvalue_2))
  (Default|SetMerchant _output_get self)
  (UserInterface|Viewport|AddtoViewport _output_get 0)
  ;[1 1 1] 마우스 조작 설정, Input Mode 설정
  (Input|SetInputModeUIOnly _returnvalue _output_get "DoNotLock" false)
  (Variables|/Script/Engine.PlayerController|SetbShowMouseCursor _returnvalue true)
  ;[1 1 1] 카메라, 뷰타겟 지정
  (Game|Player|SetViewTargetwithBlend _returnvalue self 0.0 "VTBlend_Linear" 0.0 false)
  (CallFunction|SetCameraDefault)
  (Variables|Default|SetState "Open") ; 애니메이션 State 지정
)

(fn PreviewItemClear
  (Rendering|SetVisibility (Variables|Default|GetItemMesh) false false))