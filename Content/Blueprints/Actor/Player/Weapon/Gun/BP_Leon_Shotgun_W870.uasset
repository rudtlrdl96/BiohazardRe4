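; BP_Leon_Shotgun_W870 is Leon's W870 shotgun weapon Blueprint, handling the ejection of spent shells.
; A SpawnShell event spawns a BP_ShotgunEmptyShell at an offset behind and to the right of the gun, matching its rotation.
; It then applies a small backward impulse to the shell's mesh.
; BeginPlay, Tick, overlap and the construction script are empty.
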(event EventBeginPlay)

(event Collision|EventActorBeginOverlap
  (params (OtherActor :type Actor%20Object%20Reference)))

(event EventTick
  (params (DeltaSeconds :type Float%20%28single-precision%29)))

(event EventSpawnShell
  (bind _returnvalue (Transformation|GetActorTransform))
  (bind _returnvalue_2 (Game|SpawnActorfromClass "/Game/Blueprints/Actor/Player/Weapon/Gun/BP_ShotgunEmptyShell.BP_ShotgunEmptyShell_C" (Math|Transform|MakeTransform (+ (+ (.location _returnvalue) "") (* (Transformation|GetActorForwardVector) -15.0) (* (Transformation|GetActorRightVector) 1e+01)) (.rotation _returnvalue) "1.000000,1.000000,1.000000") "Undefined" "MultiplyWithRoot" 0 0))
  (Physics|AddImpulse (Variables|/Script/Engine.StaticMeshActor|GetStaticMeshComponent _returnvalue_2) (* (Transformation|GetActorForwardVector) -4.0) "None" false))

(fn ConstructionScript)